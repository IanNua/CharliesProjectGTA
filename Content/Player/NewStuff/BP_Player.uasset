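; BP_Player is the player character or pawn that walks around and can take control of a car.
; On BeginPlay it adds an Enhanced Input mapping context, and two axis actions drive movement along fixed world X and Y, independent of facing.
; Interact possesses CurrentCarRef and destroys the player when InteractableRange is true, otherwise printing a debug message.
; Neither of those variables is set within this Blueprint's graphs.
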(event Input|EnhancedActionEvents|EnhancedInputActionIA_Interact
  (params (ActionValue :type Boolean) (ElapsedSeconds :type Float%20%28double-precision%29) (TriggeredSeconds :type Float%20%28double-precision%29) (InputAction :type Input%20Action%20Object%20Reference :default "/Game/Input/IA_Interact.IA_Interact"))
  (if (Variables|Default|GetInteractableRange?)
    (Pawn|Possess (Game|GetPlayerController 0) (Variables|Default|GetCurrentCarRef))
    (Actor|DestroyActor)
    (else
      (Development|PrintString "No collision"))))

(event Input|EnhancedActionEvents|EnhancedInputActionIA_RightLeft
  (params (ActionValue :type Float%20%28double-precision%29) (ElapsedSeconds :type Float%20%28double-precision%29) (TriggeredSeconds :type Float%20%28double-precision%29) (InputAction :type Input%20Action%20Object%20Reference :default "/Game/Input/IA_RightLeft.IA_RightLeft"))
  (CallFunction|WalkingRL ActionValue))

(event Input|EnhancedActionEvents|EnhancedInputActionIA_ForwardBackwards
  (params (ActionValue :type Float%20%28double-precision%29) (ElapsedSeconds :type Float%20%28double-precision%29) (TriggeredSeconds :type Float%20%28double-precision%29) (InputAction :type Input%20Action%20Object%20Reference :default "/Game/Input/IA_ForwardBackwards.IA_ForwardBackwards"))
  (CallFunction|WalkingFB ActionValue))

(event EventBeginPlay
  (Input|AddMappingContext (PlayerController|LocalPlayerSubsystems|GetEnhancedInputLocalPlayerSubsystem (Game|GetPlayerController 0)) 0 0 "(bIgnoreAllPressedKeysUntilRelease=True,bForceImmediately=False,bNotifyUserSettings=False)"))

(event Collision|EventActorBeginOverlap
  (params (OtherActor :type Actor%20Object%20Reference)))

(event EventTick
  (params (DeltaSeconds :type Float%20%28single-precision%29)))

(fn ConstructionScript)

(fn WalkingFB
  (params (ScaleValue :type Float%20%28single-precision%29))
  (Pawn|Input|AddMovementInput "1.000000,0.000000,0.000000" ScaleValue false))

(fn WalkingRL
  (params (ScaleValue :type Float%20%28single-precision%29))
  (Pawn|Input|AddMovementInput "0.000000,1.000000,0.000000" ScaleValue false))