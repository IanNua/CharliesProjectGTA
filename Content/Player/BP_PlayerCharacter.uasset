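; BP_PlayerCharacter is a drivable vehicle that BP_Player can approach, with Enhanced Input for movement, exiting and pausing.
; Its VehiclePlane takes a texture through a dynamic material and turns toward the last velocity using frame-rate-independent exponential smoothing.
; Box overlaps give BP_Player a car reference and toggle its interact range.
; Interact spawns and possesses a new BP_Player; Pause opens WBP_Pause in UI-only input mode.
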(event OnComponentBeginOverlap(Box)
  (params (OverlappedComponent :type Primitive%20Component%20Object%20Reference) (OtherActor :type Actor%20Object%20Reference) (OtherComp :type Primitive%20Component%20Object%20Reference) (OtherBodyIndex :type Integer) (bFromSweep :type Boolean) (SweepResult :type Hit%20Result%20Structure%20%28by%20ref%29))
  (bind _asbp_player (Utilities|Casting|CastToBP_Player OtherActor))
  (Variables|/Game/Player/NewStuff/BP_Player.BP_Player_C|SetCurrentCarRef _asbp_player self)
  (Variables|/Game/Player/NewStuff/BP_Player.BP_Player_C|SetInteractableRange? _asbp_player true))

(event OnComponentEndOverlap(Box)
  (params (OverlappedComponent :type Primitive%20Component%20Object%20Reference) (OtherActor :type Actor%20Object%20Reference) (OtherComp :type Primitive%20Component%20Object%20Reference) (OtherBodyIndex :type Integer))
  (bind _asbp_player (Utilities|Casting|CastToBP_Player OtherActor))
  (Variables|/Game/Player/NewStuff/BP_Player.BP_Player_C|SetCurrentCarRef _asbp_player self)
  (Variables|/Game/Player/NewStuff/BP_Player.BP_Player_C|SetInteractableRange? _asbp_player false))

(event Input|EnhancedActionEvents|EnhancedInputActionIA_Move
  (params (ActionValue :type Vector%202D%20Structure) (ElapsedSeconds :type Float%20%28double-precision%29) (TriggeredSeconds :type Float%20%28double-precision%29) (InputAction :type Input%20Action%20Object%20Reference :default "/Game/Input/IA_Move.IA_Move"))
  (bind (_x _y) (Math|Vector2D|BreakVector2D ActionValue))
  (Pawn|Input|AddMovementInput (Transformation|GetActorForwardVector) _x false)
  (Pawn|Input|AddMovementInput (* (Transformation|GetActorRightVector) -1.0) _y false))

(event Input|EnhancedActionEvents|EnhancedInputActionIA_Interact
  (params (ActionValue :type Boolean) (ElapsedSeconds :type Float%20%28double-precision%29) (TriggeredSeconds :type Float%20%28double-precision%29) (InputAction :type Input%20Action%20Object%20Reference :default "/Game/Input/IA_Interact.IA_Interact"))
  (bind _mesh (Variables|Character|GetMesh))
  (bind _returnvalue (Transformation|GetWorldTransform _mesh))
  (bind _returnvalue_2 (Game|SpawnActorfromClass "/Game/Player/NewStuff/BP_Player.BP_Player_C" (Math|Transform|MakeTransform (.location _returnvalue) "0, 0, 0" (.scale _returnvalue)) "Undefined" "MultiplyWithRoot" 0 0))
  (Pawn|Possess (Game|GetPlayerController 0) _returnvalue_2))

(event Input|EnhancedActionEvents|EnhancedInputActionIA_Pause
  (params (ActionValue :type Boolean) (ElapsedSeconds :type Float%20%28double-precision%29) (TriggeredSeconds :type Float%20%28double-precision%29) (InputAction :type Input%20Action%20Object%20Reference :default "/Game/Input/IA_Pause.IA_Pause"))
  (bind _returnvalue (Game|GetPlayerController 0))
  (Game|SetGamePaused true)
  (bind _returnvalue_2 (UserInterface|CreateWidget "/Game/UI/WBP_Pause.WBP_Pause_C"))
  (UserInterface|Viewport|AddtoViewport _returnvalue_2 0)
  (Input|SetInputModeUIOnly _returnvalue 0 "DoNotLock" false)
  (Variables|/Script/Engine.PlayerController|SetbShowMouseCursor _returnvalue true))

(event EventTick
  (params (DeltaSeconds :type Float%20%28single-precision%29))
  (bind _returnvalue (Transformation|GetActorLocation))
  (bind _returnvalue_2 (Transformation|GetVelocity))
  (bind _vehicleplane (Variables|Default|GetVehiclePlane))
  (if (> (Math|Vector|VectorLength _returnvalue_2) 0.1)
    (bind _output_get (Variables|Default|SetLastVelocity _returnvalue_2))
    (Development|PrintText (Utilities|Text|FormatText "New Velocity: {Vel}" (Utilities|String|ToString(Vector) _output_get))))
  (Transformation|SetRelativeRotation _vehicleplane (Math|Rotator|Lerp(Rotator) (Variables|/Script/Engine.SceneComponent|GetRelativeRotation _vehicleplane) (Math|Rotator|FindLookatRotation _returnvalue (+ _returnvalue (Variables|Default|GetLastVelocity))) (- 1.0 (Class|KismetMathLibrary|Exp (* -8.0 DeltaSeconds))) true) false false))

(event EventBeginPlay
  (bind _returnvalue (Rendering|Material|CreateDynamicMaterialInstance "/Game/M_Vehicle.M_Vehicle" "Daddy" "None" :!class /Script/Engine.KismetMaterialLibrary))
  (Rendering|Material|SetMaterial (Variables|Default|GetVehiclePlane) 0 _returnvalue)
  (Rendering|Material|SetTextureParameterValue _returnvalue "Texture" (Variables|Default|GetCurrentTexture)))

(fn ConstructionScript)