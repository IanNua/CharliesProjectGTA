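; AC_Quest is a quest component that puts the current quest and its timer on screen.
; On BeginPlay, if no quest widget exists yet, it creates WBP_CurrentQuest with a reference to the player's BP_PlayerCharacter and adds it to the viewport.
; It checks the widget's QuestTimer once, immediately afterward; at zero, it destroys itself, removes the widget and forces garbage collection.
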(event EventBeginPlay
  ;[0 0.8829 1 0.7043] Shows quest on screen and timer for it.
  (Variables|Default|GetQuestRef
    (:then)
    (:else
      (bind _asbp_player_character (Utilities|Casting|CastToBP_PlayerCharacter (Game|GetPlayerCharacter 0)))
      (bind _returnvalue (UserInterface|CreateWidget "/Game/BP/Quests/WBP_CurrentQuest.WBP_CurrentQuest_C" 0 _asbp_player_character))
      (bind _output_get (Variables|Default|SetQuestRef _returnvalue))
      (UserInterface|Viewport|AddtoViewport _output_get 0)
      (if (== (Variables|/Game/BP/Quests/WBP_CurrentQuest.WBP_CurrentQuest_C|GetQuestTimer (Variables|Default|GetQuestRef)) 0.0)
        (Components|DestroyComponent)
        (Widget|RemovefromParent (Variables|Default|GetQuestRef))
        (Utilities|Platform|CollectGarbage)))))