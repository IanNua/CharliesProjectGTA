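; BP_CarManager spawns the AI cars from a data table when play begins.
; It loops over the names returned by GetDataTableColumnNames, prints each and uses it as a row name for lookup.
; Each found row spawns a BP_VehicleAI at its start tile actor's location with zero rotation, passing that tile, its max speed and car style material to the vehicle.
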(event EventBeginPlay
  (bind _datatable (Variables|Default|GetDataTable))
  (bind _outcolumnnames (Class|DataTableFunctionLibrary|GetDataTableColumnNames _datatable))
  (for _array_element _outcolumnnames
    (Development|PrintString (Utilities|String|ToString(Name) _array_element) true true "(R=1.000000,G=0.000000,B=0.132255,A=1.000000)")
    (bind _returnvalue (Utilities|GetDataTableRow _datatable _array_element)
      (:then
        (bind _returnvalue_2 (Game|SpawnActorfromClass "/Game/BP/AI/BP_VehicleAI.BP_VehicleAI_C" (Math|Transform|MakeTransform (Transformation|GetActorLocation (.StartLocation (Utilities|Struct|BreakF_CarType _returnvalue)))) "Undefined" "MultiplyWithRoot" 0 (.StartLocation (Utilities|Struct|BreakF_CarType _returnvalue)) (.MaxSpeed (Utilities|Struct|BreakF_CarType _returnvalue)) 0))
        (Variables|/Game/BP/AI/BP_VehicleAI.BP_VehicleAI_C|SetCurrentTile _returnvalue_2 (.StartLocation (Utilities|Struct|BreakF_CarType _returnvalue)))
        (Variables|/Game/BP/AI/BP_VehicleAI.BP_VehicleAI_C|SetMaxCarSpeedValue _returnvalue_2 (.MaxSpeed (Utilities|Struct|BreakF_CarType _returnvalue)))
        (Variables|/Game/BP/AI/BP_VehicleAI.BP_VehicleAI_C|SetMaterial _returnvalue_2 (.CarStyle (Utilities|Struct|BreakF_CarType _returnvalue)))))))

(event Collision|EventActorBeginOverlap
  (params (OtherActor :type Actor%20Object%20Reference)))

(event EventTick
  (params (DeltaSeconds :type Float%20%28single-precision%29)))

(fn ConstructionScript)