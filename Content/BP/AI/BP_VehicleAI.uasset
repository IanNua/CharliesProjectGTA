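; BP_VehicleAI is a vehicle actor that drives itself along lane splines from one road tile to the next.
; Each tick it advances a distance by its speed and snaps its location and rotation to that point on the current spline.
; Past the spline's end it takes the tile's next tile at index 0, fetches its forward lane 0 spline and restarts the distance at zero.
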(event Custom|UpdateProgress
  (params (DeltaTime :type Float%20%28double-precision%29))
  (bind _currentspline (Variables|Default|GetCurrentSpline))
  (bind _output_get (Variables|Default|SetProgressDistance (+ (Variables|Default|GetProgressDistance) (* DeltaTime (Variables|Default|GetSpeed)))))
  (Transformation|SetActorLocation (Math|Vector|MakeVector (.x (.location (Spline|GetTransformatDistanceAlongSpline _currentspline _output_get "World" false))) (.y (.location (Spline|GetTransformatDistanceAlongSpline _currentspline _output_get "World" false))) (.z (.location (Spline|GetTransformatDistanceAlongSpline _currentspline _output_get "World" false)))) false false)
  (Transformation|SetActorRotation (.rotation (Spline|GetTransformatDistanceAlongSpline _currentspline _output_get "World" false)))
  (if (> _output_get (Spline|GetSplineLength _currentspline))
    (Development|PrintString "Reached end of spline!")
    (bind _out_tile (Default|GetNextTile (Variables|Default|GetCurrentTile)))
    (CallFunction|SetNewTile _out_tile)))

(event Custom|SetNewTile
  (params (New%20Tile :type BP%20Tile%20Base%20Object%20Reference))
  (bind _output_get (Variables|Default|SetCurrentTile New%20Tile))
  (bind _spline (Default|GetSpline New%20Tile 0 false))
  (Variables|Default|SetCurrentSpline _spline)
  (Variables|Default|SetProgressDistance 0.0))

(event EventTick
  (params (DeltaSeconds :type Float%20%28single-precision%29))
  (CallFunction|UpdateProgress DeltaSeconds))

(event EventBeginPlay
  (CallFunction|SetNewTile (Variables|Default|GetCurrentTile)))

(fn ConstructionScript
  (Rendering|Material|SetMaterial (Variables|Default|GetVehiclePlane1) 0 "/Game/M_Vehicle.M_Vehicle"))